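; Procedural floor Blueprint that builds an NUnitsX by NUnitsY grid of floor tiles in the Construction Script, with optional roof meshes and point lights.
; Tile spacing comes from the measured bounds of the previously placed floor mesh, which also yields the overall room size.
; Each light takes its properties from a per-tile LightArray, which grows with defaults as needed and is cleared when lights are disabled.
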(event EventBeginPlay)

(event Collision|EventActorBeginOverlap
  (params (OtherActor :type Actor%20Object%20Reference)))

(event EventTick
  (params (DeltaSeconds :type Float%20%28single-precision%29)))

(fn ConstructionScript
  (Variables|FloorGeometry|SetCounter 0)
  (for _index (range 1 (Variables|FloorGeometry|GetNUnitsY))
    (for _index_2 (range 1 (Variables|FloorGeometry|GetNUnitsX))
      (bind _transform (CallFunction|CalculateUnitFloorPosition _index_2 _index (Variables|FloorGeometry|GetXSPrevious) (Variables|FloorGeometry|GetYSPrevious)))
      (bind _returnvalue (AddComponent|AddStaticMeshComponent false _transform))
      (Components|StaticMesh|SetStaticMesh _returnvalue (Utilities|ResolveSoftReference (Variables|FloorMesh|GetFloor%20Mesh)))
      ;[1 1 1] Roof
      (if (Variables|Roof|GetBuild%20Roof)
        (bind _returnvalue_2 (AddComponent|AddStaticMeshComponent false (Math|Transform|ComposeTransforms _transform (Math|Transform|MakeTransform (Math|Vector|MakeVector 0.0 0.0 (Variables|Roof|GetHeight))))))
        (Components|StaticMesh|SetStaticMesh _returnvalue_2 (Utilities|ResolveSoftReference (Variables|Roof|GetRoof%20Mesh))))
      (bind (_xs _ys) (CallFunction|CalculateStaticMeshDimensions _returnvalue))
      (Variables|FloorGeometry|SetXSPrevious _xs)
      (Variables|FloorGeometry|SetYSPrevious _ys)
      ;[1 1 1] Light
      (if (Variables|Lights|GetAdd%20Light)
        (Math|Integer|CompareInt (Variables|FloorGeometry|GetCounter) (Utilities|Array|LastIndex (Variables|Lights|GetLightArray))
          (:>
            (Utilities|Array|Add (Variables|Lights|GetLightArray) (Variables|Lights|GetDefault%20Light%20Properties)))
          (:==
            _)
          (:<
            _))
        (bind _returnvalue_3 (AddComponent|AddPointLightComponent false (Math|Transform|ComposeTransforms _transform (Math|Transform|MakeTransform (Math|Vector|MakeVector (/ (Variables|FloorGeometry|GetXSPrevious) 2.0) (/ (Variables|FloorGeometry|GetYSPrevious) 2.0) (.Height (Utilities|Struct|BreakFloorLightProperties (Utilities|Array|Get(acopy) (Variables|Lights|GetLightArray) (Variables|FloorGeometry|GetCounter)))))))))
        (Rendering|Components|Light|SetIntensity _returnvalue_3 (.Intensity (Utilities|Struct|BreakFloorLightProperties (Utilities|Array|Get(acopy) (Variables|Lights|GetLightArray) (Variables|FloorGeometry|GetCounter)))))
        (Rendering|Lighting|SetAttenuationRadius _returnvalue_3 (.AttenuationR (Utilities|Struct|BreakFloorLightProperties (Utilities|Array|Get(acopy) (Variables|Lights|GetLightArray) (Variables|FloorGeometry|GetCounter)))))
        (Rendering|Components|Light|SetLightColor _returnvalue_3 (.Color (Utilities|Struct|BreakFloorLightProperties (Utilities|Array|Get(acopy) (Variables|Lights|GetLightArray) (Variables|FloorGeometry|GetCounter)))) true)
        (else
          (Utilities|Array|Clear (Variables|Lights|GetLightArray))))
      ;[1 1 1] End Of Loop
      (Math|Integer|IncrementInt (Variables|FloorGeometry|GetCounter)
        (:%20%20
          (Variables|FloorGeometry|SetRoomXS (* (Variables|FloorGeometry|GetNUnitsX) (Variables|FloorGeometry|GetXSPrevious)))
          (Variables|FloorGeometry|SetRoomYS (* (Variables|FloorGeometry|GetNUnitsY) (Variables|FloorGeometry|GetYSPrevious))))))))

(fn CalculateUnitFloorPosition
  (params (XUnit :type Integer) (YUnit :type Integer) (UnitFloorSizeX :type Float%20%28single-precision%29) (UnitFloorSizeY :type Float%20%28single-precision%29))
  (return (Math|Transform|MakeTransform (Math|Vector|MakeVector (|((x-1)*xs) XUnit UnitFloorSizeX) (|((x-1)*xs) YUnit UnitFloorSizeY) 0.0))))

(fn CalculateStaticMeshDimensions
  (params (StaticMeshClassReference :type Static%20Mesh%20Component%20Object%20Reference))
  (bind _boxextent (Collision|GetComponentBounds StaticMeshClassReference))
  (bind _returnvalue (* _boxextent 2))
  (bind (_x _y _z) (Math|Vector|BreakVector _returnvalue))
  (return _x _y _z))