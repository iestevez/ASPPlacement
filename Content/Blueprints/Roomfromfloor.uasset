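; Room Blueprint that builds a rectangular ring of modular walls in the Construction Script from a list of wall descriptions.
; Each entry adds a plain, window or door mesh, with transform and side (A–D) derived from its index and the unit counts.
; A running offset records each wall's position along its side.
; When enabled, a second pass shifts per-wall and optional per-type constraints by that offset and groups them by side.
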(event EventBeginPlay)

(event Collision|EventActorBeginOverlap
  (params (OtherActor :type Actor%20Object%20Reference)))

(event EventTick
  (params (DeltaSeconds :type Float%20%28single-precision%29)))

(fn ConstructionScript
  (bind _room_constraints (Variables|RoomConstraints|GetRoom%20Constraints))
  (bind _list_of_walls (Variables|Walls|GetList%20of%20walls))
  (|CallParentFunction)
  ;[1 1 1] Wall Placement
  (for (_array_element _array_index) _list_of_walls
    (switch Utilities|FlowControl|Switch|SwitchonWallTypes (.WallType (Utilities|Struct|BreakWallDescription _array_element))
      (:NewEnumerator0
        (Variables|Walls|SetSMToWall (Utilities|ResolveSoftReference (Variables|Walls|GetWallWithoutDoor))))
      (:NewEnumerator1
        (Variables|Walls|SetSMToWall (Utilities|ResolveSoftReference (Variables|Walls|GetWallWithWindows))))
      (:NewEnumerator2
        (Variables|Walls|SetSMToWall (Utilities|ResolveSoftReference (Variables|Walls|GetWallWithDoor)))))
    (bind _returnvalue (AddComponent|AddStaticMeshComponent false (.Wall%20Transform (Walls|CalculateWallTransform _array_index (Variables|Default|GetNUnitsX) (Variables|Default|GetNUnitsY) (Variables|Default|GetXSPrevious) (Variables|Default|GetYSPrevious) (Variables|Walls|GetWallOffset)))))
    (Components|StaticMesh|SetStaticMesh _returnvalue (Variables|Walls|GetSMToWall))
    (bind _offset (Walls|CalculateNewOffset (LocalVariables|GetPreviousOrientation) (.Wall%20Orientation (Walls|CalculateWallTransform _array_index (Variables|Default|GetNUnitsX) (Variables|Default|GetNUnitsY) (Variables|Default|GetXSPrevious) (Variables|Default|GetYSPrevious) (Variables|Walls|GetWallOffset))) (LocalVariables|GetPreviousWallSize) (LocalVariables|GetPreviousOffset)))
    (Utilities|Array|SetArrayElem _list_of_walls _array_index (Utilities|Struct|MakeWallDescription (.WallType (Utilities|Struct|BreakWallDescription _array_element)) (.Constraints (Utilities|Struct|BreakWallDescription _array_element)) (.UseGeneralConstraints (Utilities|Struct|BreakWallDescription _array_element)) (.Wall%20Orientation (Walls|CalculateWallTransform _array_index (Variables|Default|GetNUnitsX) (Variables|Default|GetNUnitsY) (Variables|Default|GetXSPrevious) (Variables|Default|GetYSPrevious) (Variables|Walls|GetWallOffset))) _offset))
    (LocalVariables|SetPreviousOrientation (.Wall%20Orientation (Walls|CalculateWallTransform _array_index (Variables|Default|GetNUnitsX) (Variables|Default|GetNUnitsY) (Variables|Default|GetXSPrevious) (Variables|Default|GetYSPrevious) (Variables|Walls|GetWallOffset))))
    (LocalVariables|SetPreviousWallSize (.WallLength (Walls|CalculateWallTransform _array_index (Variables|Default|GetNUnitsX) (Variables|Default|GetNUnitsY) (Variables|Default|GetXSPrevious) (Variables|Default|GetYSPrevious) (Variables|Walls|GetWallOffset))))
    (LocalVariables|SetPreviousOffset _offset))
  ;[1 1 1] Generate Constraint Array
  (if (Variables|RoomConstraints|GetObtainConst)
    (RoomConstraints|ClearRoomConstraints _room_constraints)
    (for _array_element_2 (Variables|Walls|GetList%20of%20walls)
      (Utilities|Array|Clear (Variables|RoomConstraints|GetTemporal%20Array%20of%20Constraints))
      (Utilities|Array|AppendArray (Variables|RoomConstraints|GetTemporal%20Array%20of%20Constraints) (.Constraints (Utilities|Struct|BreakWallDescription _array_element_2)))
      (if (.UseGeneralConstraints (Utilities|Struct|BreakWallDescription _array_element_2))
        (bind _constraintarray (RoomConstraints|SelectWallTypeGeneralConstraints (Variables|RoomConstraints|GetGeneral%20Wall%20Constraints) (.WallType (Utilities|Struct|BreakWallDescription _array_element_2))))
        (Utilities|Array|AppendArray (Variables|RoomConstraints|GetTemporal%20Array%20of%20Constraints) _constraintarray))
      (bind _newconstraints (RoomConstraints|AddOffsettoConstraints (.Offset (Utilities|Struct|BreakWallDescription _array_element_2)) (Variables|RoomConstraints|GetTemporal%20Array%20of%20Constraints)))
      (Variables|RoomConstraints|SetTemporal%20Array%20of%20Constraints _newconstraints)
      (RoomConstraints|SetRoomConstraints (.WallOrientation (Utilities|Struct|BreakWallDescription _array_element_2)) (Variables|RoomConstraints|GetRoom%20Constraints) (Variables|RoomConstraints|GetTemporal%20Array%20of%20Constraints)))
    (else
      (RoomConstraints|ClearRoomConstraints _room_constraints))))

(fn CalculateWallTransform
  (params (Wall%20Index :type Integer) (NUX :type Integer) (NUY :type Integer) (XS :type Float%20%28single-precision%29) (YS :type Float%20%28single-precision%29) (WT :type Float%20%28single-precision%29))
  (bind _returnvalue (|((K%(NX+NY))-(NX-1)) Wall%20Index NUX NUY))
  (LocalVariables|SetLWT WT)
  (Math|Integer|CompareInt (|((K/(NX+NY))%2) Wall%20Index NUX NUY) 0
    (:>
      (Math|Integer|CompareInt _returnvalue 0
        (:>
          (return (Math|Transform|MakeTransform (Math|Vector|MakeVector (|(0-{769FB911-47EE-7E03-5119-5F812F9B9BB5})) (|((NY-K)*YS) (|(Y-1) _returnvalue) YS NUY) 0.0) "0,-90.000000, 0" "1.000000,1,1") "WallD" YS))
        (:==
          _)
        (:<
          _))
      (return (Math|Transform|MakeTransform (Math|Vector|MakeVector (|((NX-K)*XS) NUX (|((NX-1)+x) _returnvalue NUX) XS) (|(YS+{769FB911-47EE-7E03-5119-5F812F9B9BB5}) (|(N*S) NUY YS)) 0.0) "0,180.000000, 0" "1.000000,1,1") "WallC" XS))
    (:==
      _)
    (:<
      _))
  (Math|Integer|CompareInt _returnvalue 0
    (:>
      (return (Math|Transform|MakeTransform (Math|Vector|MakeVector (|(XS+{769FB911-47EE-7E03-5119-5F812F9B9BB5}) (|(N*S) NUX XS)) (|(K*YS) (|(Y-1) _returnvalue) YS) 0.0) "0,90.000000, 0" "1.000000,1,1") "WallB" YS))
    (:==
      _)
    (:<
      _))
  (return (Math|Transform|MakeTransform (Math|Vector|MakeVector (|(K*XS) (|(X+(NX-1)) _returnvalue NUX) XS) (* -1 (LocalVariables|GetLWT)) 0.0) "0,0.000000, 0") "WallA" XS))

(fn SelectWallOrientationArray
  (params (RoomConstraints :type Room%20Constraints%20Structure%20%28by%20ref%29) (RoomFace :type FEWalls%20Enum))
  (bind (_walla _wallb _wallc _walld) (Utilities|Struct|BreakRoomConstraints RoomConstraints))
  (switch Utilities|FlowControl|Switch|SwitchonFEWalls RoomFace
    (:WallA
      _)
    (:WallB
      (return _wallb))
    (:WallC
      (return _wallc))
    (:WallD
      (return _walld))
    (:None
      _))
  (return _walla))

(fn SelectWallTypeGeneralConstraints
  (params (GeneralConstraints :type General%20Constraints%20Structure) (WallType :type WallTypes%20Enum))
  (bind (_basicwall _wallwithwindow _wallwithdoor) (Utilities|Struct|BreakGeneralConstraints GeneralConstraints))
  (switch Utilities|FlowControl|Switch|SwitchonWallTypes WallType
    (:NewEnumerator0
      (return _basicwall))
    (:NewEnumerator1
      (return _wallwithwindow))
    (:NewEnumerator2
      (return _wallwithdoor))))

(fn SetRoomConstraints
  (params (Room%20Face :type FEWalls%20Enum) (Room%20Contraints%20Reference :type Room%20Constraints%20Structure%20%28by%20ref%29) (Constraints :type Array%20of%20Vectors))
  (bind (_walla _wallb _wallc _walld) (Utilities|Struct|BreakRoomConstraints Room%20Contraints%20Reference))
  (switch Utilities|FlowControl|Switch|SwitchonFEWalls Room%20Face
    (:WallA
      (Utilities|Array|AppendArray _walla Constraints))
    (:WallB
      (Utilities|Array|AppendArray _wallb Constraints))
    (:WallC
      (Utilities|Array|AppendArray _wallc Constraints))
    (:WallD
      (Utilities|Array|AppendArray _walld Constraints))))

(fn ClearRoomConstraints
  (params (Room%20Contraints%20Reference :type Room%20Constraints%20Structure%20%28by%20ref%29))
  (bind _emptyconstraintsarray (Variables|RoomConstraints|GetEmptyConstraintsArray))
  (Utilities|Struct|SetmembersinRoomConstraints Room%20Contraints%20Reference _emptyconstraintsarray _emptyconstraintsarray _emptyconstraintsarray _emptyconstraintsarray))

(fn CalculateNewOffset
  (params (PreviousOrientation :type FEWalls%20Enum) (NewOrientation :type FEWalls%20Enum) (PreviousWallSize :type Float%20%28single-precision%29) (PreviousOffset :type Float%20%28single-precision%29))
  (if (Utilities|Enum|Equal(Enum) PreviousOrientation NewOrientation)
    (return (+ PreviousWallSize PreviousOffset))
    (else
      (return 0.0))))

(fn AddOffsettoConstraints
  (params (Offset :type Float%20%28single-precision%29) (Constraints :type Array%20of%20Vectors))
  (for _array_element Constraints
    (Utilities|Array|Add (LocalVariables|GetTempArray) (+ _array_element Offset)))
  (return (LocalVariables|GetTempArray)))