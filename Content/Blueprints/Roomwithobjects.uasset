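; Room actor that furnishes itself with static meshes along four walls (A–D) in its construction script, on top of its parent's script.
; With AutomaticGeneration on, flattened per-wall constraints feed Placement, which rebuilds the object list.
; Each object's position derives from wall, corner distance, rotation and scaled mesh bounds.
; Spawned mesh components are then rotated and shifted using their Point1/Point2 sockets to align footprint corners.
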(event EventBeginPlay)

(event Collision|EventActorBeginOverlap
  (params (OtherActor :type Actor%20Object%20Reference)))

(event EventTick
  (params (DeltaSeconds :type Float%20%28single-precision%29)))

(fn ConstructionScript
  (|CallParentFunction)
  ;[1 1 1] Automatic Placement
  (if (Variables|Objects|GetAutomatic_Generation)
    (bind _list_of_wall_constraints (CallFunction|FlatRoomConstraints (Variables|Default|GetRoom%20Constraints)))
    (bind _newlobjects (Class|ObjectProceduralFunctionLibrary|Placement (Variables|Objects|GetUnit) (Variables|Walls|GetWall%20Width) (Variables|Default|GetRoomXS) (Variables|Default|GetRoomYS) (Variables|Objects|GetList%20of%20objects) _list_of_wall_constraints))
    (Variables|Objects|SetList%20of%20objects _newlobjects))
  ;[1 1 1] Calculo de la posicion
  (for (_array_element _array_index) (Variables|Objects|GetList%20of%20objects)
    (bind _dimensions (CallFunction|GetStaticMeshDimensions (.StaticMesh (Utilities|Struct|BreakSObjectDescription _array_element))))
    (bind _position (CallFunction|CalculatePositionfromWBA (.wall (Utilities|Struct|BreakSObjectDescription _array_element)) (.distanceFromLeftCorner (Utilities|Struct|BreakSObjectDescription _array_element)) (Variables|Default|GetRoomXS) (Variables|Default|GetRoomYS) (.rotation (Utilities|Struct|BreakSObjectDescription _array_element)) (.X (Math|Vector|BreakVector (* _dimensions (.scale (Utilities|Struct|BreakSObjectDescription _array_element))))) (.Y (Math|Vector|BreakVector (* _dimensions (.scale (Utilities|Struct|BreakSObjectDescription _array_element))))) (Variables|Objects|GetUnit) (Variables|Walls|GetWall%20Width)))
    (bind _objectfacetowall (CallFunction|FacetoWall (.wall (Utilities|Struct|BreakSObjectDescription _array_element)) (.rotation (Utilities|Struct|BreakSObjectDescription _array_element))))
    (bind _structout (Utilities|Struct|SetmembersinSObjectDescription _array_element _dimensions _position _objectfacetowall))
    (Utilities|Array|SetArrayElem (Variables|Objects|GetList%20of%20objects) _array_index _structout))
  ;[1 1 1] Add SM Component
  (for _array_element_2 (Variables|Objects|GetList%20of%20objects)
    (bind _returnvalue (AddComponent|AddStaticMeshComponent false (Math|Transform|MakeTransform (.position (Utilities|Struct|BreakSObjectDescription _array_element_2)) "0, 0, 0" "1.000000,1.000000,1.000000")))
    (LocalVariables|SetSM_Compref _returnvalue)
    (Components|StaticMesh|SetStaticMesh (LocalVariables|GetSM_Compref) (.StaticMesh (Utilities|Struct|BreakSObjectDescription _array_element_2)))
    (CallFunction|GetRotationfromSockets (.rotation (Utilities|Struct|BreakSObjectDescription _array_element_2)) (LocalVariables|GetSM_Compref))
    (bind _asinstanced_static_mesh_component (Utilities|Casting|CastToInstancedStaticMeshComponent _returnvalue))
    (Utilities|Array|Add (Variables|Default|GetListOfStaticMeshComponents) _asinstanced_static_mesh_component)))

(fn CalculatePositionfromWBA
  (params (RoomFace :type FEWalls%20Enum) (Distance :type Integer) (XSize :type Float%20%28single-precision%29) (YSize :type Float%20%28single-precision%29) (Rotation :type FEFaces%20Enum) (OXSize :type Float%20%28single-precision%29) (OYSize :type Float%20%28single-precision%29) (Unit :type Float%20%28single-precision%29) (Width :type Float%20%28single-precision%29))
  (bind _returnvalue (/ OYSize 1.0))
  (bind _returnvalue_2 (/ OXSize 1.0))
  (bind _returnvalue_3 (* Distance Unit))
  (LocalVariables|SetLWidth Width)
  (switch Utilities|FlowControl|Switch|SwitchonFEFaces Rotation
    (:WallA
      ;[1 1 1] Objects dimensions after rotation
      (LocalVariables|SetLh _returnvalue_2 :!label _label)
      (LocalVariables|SetLv _returnvalue))
    (:WallB
      (LocalVariables|SetLh _returnvalue)
      (LocalVariables|SetLv _returnvalue_2))
    (:WallC
      (LocalVariables|SetLh _returnvalue_2)
      (LocalVariables|SetLv _returnvalue))
    (:WallD
      (LocalVariables|SetLh _returnvalue)
      (LocalVariables|SetLv _returnvalue_2))
    (:None
      (goto _label)))
  ;[1 1 1] Object position from wall face
  (switch Utilities|FlowControl|Switch|SwitchonFEWalls RoomFace
    (:WallA
      _)
    (:WallB
      (return (|(vector(((Xs-{D3498A3D-461A-80BC-41D4-5780E0C95130})-{D1F9F017-446F-2043-E425-BB919E95DB14}),Pos,0)) XSize _returnvalue_3)))
    (:WallC
      (return (|(vector((((Xs-{D3498A3D-461A-80BC-41D4-5780E0C95130})-Pos)-{D1F9F017-446F-2043-E425-BB919E95DB14}),((Ys-{D3498A3D-461A-80BC-41D4-5780E0C95130})-{6CC5E904-49CB-1C21-EE92-73AA3F93036E}),0)) XSize _returnvalue_3 YSize)))
    (:WallD
      (return (|(vector({D3498A3D-461A-80BC-41D4-5780E0C95130},(((Ys-{D3498A3D-461A-80BC-41D4-5780E0C95130})-Pos)-{6CC5E904-49CB-1C21-EE92-73AA3F93036E}),0)) YSize _returnvalue_3)))
    (:None
      _))
  (return (|(vector((Pos+{D3498A3D-461A-80BC-41D4-5780E0C95130}),{D3498A3D-461A-80BC-41D4-5780E0C95130},0)) _returnvalue_3)))

(fn FromUnits
  (params (Units :type Integer) (ConversionFactor :type Float%20%28single-precision%29))
  (return (* Units ConversionFactor)))

(fn ToUnits
  (params (Dimension :type Float%20%28single-precision%29) (ConversionFactor :type Float%20%28single-precision%29))
  (return (|(round((dim/cf))) Dimension ConversionFactor)))

(fn FacetoWall
  (params (Wall :type FEWalls%20Enum) (Rotation :type FEFaces%20Enum))
  (switch Utilities|FlowControl|Switch|SwitchonFEWalls Wall
    (:WallA
      (switch Utilities|FlowControl|Switch|SwitchonFEFaces Rotation :!label _label
        (:WallA
          _)
        (:WallB
          (return "WallB"))
        (:WallC
          (return "WallC"))
        (:WallD
          (return "WallD"))
        (:None
          _)))
    (:WallB
      (switch Utilities|FlowControl|Switch|SwitchonFEFaces Rotation
        (:WallA
          (return "WallB"))
        (:WallB
          (return "WallC"))
        (:WallC
          (return "WallD"))
        (:WallD
          _)
        (:None
          (return "WallB"))))
    (:WallC
      (switch Utilities|FlowControl|Switch|SwitchonFEFaces Rotation
        (:WallA
          (return "WallC"))
        (:WallB
          (return "WallD"))
        (:WallC
          _)
        (:WallD
          (return "WallB"))
        (:None
          (return "WallC"))))
    (:WallD
      (switch Utilities|FlowControl|Switch|SwitchonFEFaces Rotation
        (:WallA
          (return "WallD"))
        (:WallB
          _)
        (:WallC
          (return "WallB"))
        (:WallD
          (return "WallC"))
        (:None
          (return "WallD"))))
    (:None
      (goto _label)))
  (return "WallA"))

(fn GetStaticMeshDimensions
  (params (staticmesh :type Static%20Mesh%20Object%20Reference))
  (bind _returnvalue (StaticMesh|GetBoundingBox staticmesh))
  (bind (_min _max) (Utilities|Struct|BreakBox _returnvalue))
  (return (- _max _min)))

(fn GetRotationAngle
  (params (Rotation :type FEFaces%20Enum))
  (switch Utilities|FlowControl|Switch|SwitchonFEFaces Rotation
    (:WallA
      _)
    (:WallB
      (return "0.000000,90.000000, 0"))
    (:WallC
      (return "0.000000,180.000000, 0"))
    (:WallD
      (return "0.000000,270.000000, 0"))
    (:None
      _))
  (return "0, 0, 0"))

(fn FlatRoomConstraints
  (params (Room%20Constraints :type Room%20Constraints%20Structure))
  (bind (_walla _wallb _wallc _walld) (Utilities|Struct|BreakRoomConstraints Room%20Constraints))
  (Utilities|Array|Clear (LocalVariables|GetTempArray))
  (for _array_element _walla
    (Utilities|Array|Add (LocalVariables|GetTempArray) (Utilities|Struct|MakeSWallConstraint "WallA" _array_element)))
  (for _array_element_2 _wallb
    (Utilities|Array|Add (LocalVariables|GetTempArray) (Utilities|Struct|MakeSWallConstraint "WallB" _array_element_2)))
  (for _array_element_3 _wallc
    (Utilities|Array|Add (LocalVariables|GetTempArray) (Utilities|Struct|MakeSWallConstraint "WallC" _array_element_3)))
  (for _array_element_4 _walld
    (Utilities|Array|Add (LocalVariables|GetTempArray) (Utilities|Struct|MakeSWallConstraint "WallD" _array_element_4)))
  (return (LocalVariables|GetTempArray)))

(fn GetRotationfromSockets
  (params (ObjectRotation :type FEFaces%20Enum) (SM_Comp :type Static%20Mesh%20Component%20Object%20Reference))
  (bind _output_get (LocalVariables|SetLSM_Comp SM_Comp))
  (switch Utilities|FlowControl|Switch|SwitchonFEFaces ObjectRotation
    (:WallA
      _)
    (:WallB
      (Transformation|SetRelativeRotation (LocalVariables|GetLSM_Comp) (Math|Rotator|CombineRotators (Math|Rotator|CombineRotators (Class|KismetMathLibrary|NegateRotator (Math|Conversions|RotationFromXVector (- (Transformation|GetSocketLocation _output_get "Point2") (Transformation|GetSocketLocation _output_get "Point1")))) "0,45.000000, 0") "0,90.000000, 0") false false)
      (Transformation|SetWorldLocation (LocalVariables|GetLSM_Comp) (|(ObjectPosition+(ObjectPosition-P1)) (Transformation|GetWorldLocation _output_get) (Math|Vector|MakeVector (.X (Math|Vector|BreakVector (Transformation|GetSocketLocation _output_get "Point2"))) (.Y (Math|Vector|BreakVector (Transformation|GetSocketLocation _output_get "Point1"))) (.Z (Math|Vector|BreakVector (Transformation|GetSocketLocation _output_get "Point1"))))) false false)
      (return (|(ObjectPosition+(ObjectPosition-P1)) (Transformation|GetWorldLocation _output_get) (Math|Vector|MakeVector (.X (Math|Vector|BreakVector (Transformation|GetSocketLocation _output_get "Point2"))) (.Y (Math|Vector|BreakVector (Transformation|GetSocketLocation _output_get "Point1"))) (.Z (Math|Vector|BreakVector (Transformation|GetSocketLocation _output_get "Point1"))))) (Math|Rotator|CombineRotators (Math|Rotator|CombineRotators (Class|KismetMathLibrary|NegateRotator (Math|Conversions|RotationFromXVector (- (Transformation|GetSocketLocation _output_get "Point2") (Transformation|GetSocketLocation _output_get "Point1")))) "0,45.000000, 0") "0,90.000000, 0")))
    (:WallC
      (Transformation|SetRelativeRotation (LocalVariables|GetLSM_Comp) (Math|Rotator|CombineRotators (Math|Rotator|CombineRotators (Class|KismetMathLibrary|NegateRotator (Math|Conversions|RotationFromXVector (- (Transformation|GetSocketLocation _output_get "Point2") (Transformation|GetSocketLocation _output_get "Point1")))) "0,45.000000, 0") "0,180.000000, 0") false false)
      (Transformation|SetWorldLocation (LocalVariables|GetLSM_Comp) (|(ObjectPosition+(ObjectPosition-P1)) (Transformation|GetWorldLocation _output_get) (Math|Vector|MakeVector (.X (Math|Vector|BreakVector (Transformation|GetSocketLocation _output_get "Point2"))) (.Y (Math|Vector|BreakVector (Transformation|GetSocketLocation _output_get "Point2"))) (.Z (Math|Vector|BreakVector (Transformation|GetSocketLocation _output_get "Point1"))))) false false)
      (return (|(ObjectPosition+(ObjectPosition-P1)) (Transformation|GetWorldLocation _output_get) (Transformation|GetSocketLocation _output_get "Point1")) (Math|Rotator|CombineRotators (Math|Rotator|CombineRotators (Class|KismetMathLibrary|NegateRotator (Math|Conversions|RotationFromXVector (- (Transformation|GetSocketLocation _output_get "Point2") (Transformation|GetSocketLocation _output_get "Point1")))) "0,45.000000, 0") "0,180.000000, 0")))
    (:WallD
      (Transformation|SetRelativeRotation (LocalVariables|GetLSM_Comp) (Math|Rotator|CombineRotators (Math|Rotator|CombineRotators (Class|KismetMathLibrary|NegateRotator (Math|Conversions|RotationFromXVector (- (Transformation|GetSocketLocation _output_get "Point2") (Transformation|GetSocketLocation _output_get "Point1")))) "0,45.000000, 0") "0,270.000000, 0") false false)
      (Transformation|SetWorldLocation (LocalVariables|GetLSM_Comp) (|(ObjectPosition+(ObjectPosition-P1)) (Transformation|GetWorldLocation _output_get) (Math|Vector|MakeVector (.X (Math|Vector|BreakVector (Transformation|GetSocketLocation _output_get "Point1"))) (.Y (Math|Vector|BreakVector (Transformation|GetSocketLocation _output_get "Point2"))) (.Z (Math|Vector|BreakVector (Transformation|GetSocketLocation _output_get "Point1"))))) false false)
      (return (|(ObjectPosition+(ObjectPosition-P1)) (Transformation|GetWorldLocation _output_get) (Math|Vector|MakeVector (.X (Math|Vector|BreakVector (Transformation|GetSocketLocation _output_get "Point1"))) (.Y (Math|Vector|BreakVector (Transformation|GetSocketLocation _output_get "Point2"))) (.Z (Math|Vector|BreakVector (Transformation|GetSocketLocation _output_get "Point1"))))) (Math|Rotator|CombineRotators (Math|Rotator|CombineRotators (Class|KismetMathLibrary|NegateRotator (Math|Conversions|RotationFromXVector (- (Transformation|GetSocketLocation _output_get "Point2") (Transformation|GetSocketLocation _output_get "Point1")))) "0,45.000000, 0") "0,270.000000, 0")))
    (:None
      _))
  (Transformation|SetRelativeRotation (LocalVariables|GetLSM_Comp) (Math|Rotator|CombineRotators (Math|Rotator|CombineRotators (Class|KismetMathLibrary|NegateRotator (Math|Conversions|RotationFromXVector (- (Transformation|GetSocketLocation _output_get "Point2") (Transformation|GetSocketLocation _output_get "Point1")))) "0,45.000000, 0") "0, 0, 0") false false)
  (Transformation|SetWorldLocation (LocalVariables|GetLSM_Comp) (|(ObjectPosition+(ObjectPosition-P1)) (Transformation|GetWorldLocation _output_get) (Transformation|GetSocketLocation _output_get "Point1")) false false)
  (return (|(ObjectPosition+(ObjectPosition-P1)) (Transformation|GetWorldLocation _output_get) (Transformation|GetSocketLocation _output_get "Point1")) (Math|Rotator|CombineRotators (Math|Rotator|CombineRotators (Class|KismetMathLibrary|NegateRotator (Math|Conversions|RotationFromXVector (- (Transformation|GetSocketLocation _output_get "Point2") (Transformation|GetSocketLocation _output_get "Point1")))) "0,45.000000, 0") "0, 0, 0")))