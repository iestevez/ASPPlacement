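; Function library for placing static mesh objects along the four walls (A–D) of a rectangular area.
; Mesh sockets Point1, Point2 and PointF define each object's dimensions and facing direction.
; CorrectSMComponent uses them to rotate the component in 90-degree steps and shift it so a footprint corner becomes its reference point.
; CalculateReferenceCornerPosition converts wall, distance, wall width and rotated object size into a position, with CalculateFaceToWall resolving which face meets the wall.
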(fn CorrectSMComponent
  (params (ObjectRotation :type FEFaces%20Enum) (SM_Comp :type Static%20Mesh%20Component%20Object%20Reference))
  (bind (_dimensions _unitv_facea) (CallFunction|GetStaticMeshComponentDimensions SM_Comp))
  (LocalVariables|SetDimA (.X (Math|Vector|BreakVector _dimensions)))
  (LocalVariables|SetDimB (.Y (Math|Vector|BreakVector _dimensions)))
  (bind _output_get (LocalVariables|SetLSM_Comp SM_Comp))
  (switch Utilities|FlowControl|Switch|SwitchonFEFaces ObjectRotation
    (:WallA
      _)
    (:WallB
      (Transformation|SetRelativeRotation (LocalVariables|GetLSM_Comp) (Math|Rotator|CombineRotators (Math|Rotator|CombineRotators (Class|KismetMathLibrary|NegateRotator (Math|Conversions|RotationFromXVector _unitv_facea)) "0, 0, 0") "0,90.000000, 0") false false)
      (Transformation|SetWorldLocation (LocalVariables|GetLSM_Comp) (|(ObjectPosition+(ObjectPosition-P1)) (Transformation|GetWorldLocation _output_get) (Math|Vector|MakeVector (.X (Math|Vector|BreakVector (Transformation|GetSocketLocation _output_get "Point2"))) (.Y (Math|Vector|BreakVector (Transformation|GetSocketLocation _output_get "Point1"))) (.Z (Math|Vector|BreakVector (Transformation|GetSocketLocation _output_get "Point1"))))) false false)
      (return (|(ObjectPosition+(ObjectPosition-P1)) (Transformation|GetWorldLocation _output_get) (Math|Vector|MakeVector (.X (Math|Vector|BreakVector (Transformation|GetSocketLocation _output_get "Point2"))) (.Y (Math|Vector|BreakVector (Transformation|GetSocketLocation _output_get "Point1"))) (.Z (Math|Vector|BreakVector (Transformation|GetSocketLocation _output_get "Point1"))))) (Math|Rotator|CombineRotators (Math|Rotator|CombineRotators (Class|KismetMathLibrary|NegateRotator (Math|Conversions|RotationFromXVector _unitv_facea)) "0, 0, 0") "0,90.000000, 0")))
    (:WallC
      (Transformation|SetRelativeRotation (LocalVariables|GetLSM_Comp) (Math|Rotator|CombineRotators (Math|Rotator|CombineRotators (Class|KismetMathLibrary|NegateRotator (Math|Conversions|RotationFromXVector _unitv_facea)) "0, 0, 0") "0,180.000000, 0") false false)
      (Transformation|SetWorldLocation (LocalVariables|GetLSM_Comp) (|(ObjectPosition+(ObjectPosition-P1)) (Transformation|GetWorldLocation _output_get) (Math|Vector|MakeVector (.X (Math|Vector|BreakVector (Transformation|GetSocketLocation _output_get "Point2"))) (.Y (Math|Vector|BreakVector (Transformation|GetSocketLocation _output_get "Point2"))) (.Z (Math|Vector|BreakVector (Transformation|GetSocketLocation _output_get "Point1"))))) false false)
      (return (|(ObjectPosition+(ObjectPosition-P1)) (Transformation|GetWorldLocation _output_get) (Transformation|GetSocketLocation _output_get "Point1")) (Math|Rotator|CombineRotators (Math|Rotator|CombineRotators (Class|KismetMathLibrary|NegateRotator (Math|Conversions|RotationFromXVector _unitv_facea)) "0, 0, 0") "0,180.000000, 0")))
    (:WallD
      (Transformation|SetRelativeRotation (LocalVariables|GetLSM_Comp) (Math|Rotator|CombineRotators (Math|Rotator|CombineRotators (Class|KismetMathLibrary|NegateRotator (Math|Conversions|RotationFromXVector _unitv_facea)) "0, 0, 0") "0,270.000000, 0") false false)
      (Transformation|SetWorldLocation (LocalVariables|GetLSM_Comp) (|(ObjectPosition+(ObjectPosition-P1)) (Transformation|GetWorldLocation _output_get) (Math|Vector|MakeVector (.X (Math|Vector|BreakVector (Transformation|GetSocketLocation _output_get "Point1"))) (.Y (Math|Vector|BreakVector (Transformation|GetSocketLocation _output_get "Point2"))) (.Z (Math|Vector|BreakVector (Transformation|GetSocketLocation _output_get "Point1"))))) false false)
      (return (|(ObjectPosition+(ObjectPosition-P1)) (Transformation|GetWorldLocation _output_get) (Math|Vector|MakeVector (.X (Math|Vector|BreakVector (Transformation|GetSocketLocation _output_get "Point1"))) (.Y (Math|Vector|BreakVector (Transformation|GetSocketLocation _output_get "Point2"))) (.Z (Math|Vector|BreakVector (Transformation|GetSocketLocation _output_get "Point1"))))) (Math|Rotator|CombineRotators (Math|Rotator|CombineRotators (Class|KismetMathLibrary|NegateRotator (Math|Conversions|RotationFromXVector _unitv_facea)) "0, 0, 0") "0,270.000000, 0")))
    (:None
      _))
  (Transformation|SetRelativeRotation (LocalVariables|GetLSM_Comp) (Math|Rotator|CombineRotators (Math|Rotator|CombineRotators (Class|KismetMathLibrary|NegateRotator (Math|Conversions|RotationFromXVector _unitv_facea)) "0, 0, 0") "0, 0, 0") false false)
  (Transformation|SetWorldLocation (LocalVariables|GetLSM_Comp) (|(ObjectPosition+(ObjectPosition-P1)) (Transformation|GetWorldLocation _output_get) (Transformation|GetSocketLocation _output_get "Point1")) false false)
  (return (|(ObjectPosition+(ObjectPosition-P1)) (Transformation|GetWorldLocation _output_get) (Transformation|GetSocketLocation _output_get "Point1")) (Math|Rotator|CombineRotators (Math|Rotator|CombineRotators (Class|KismetMathLibrary|NegateRotator (Math|Conversions|RotationFromXVector _unitv_facea)) "0, 0, 0") "0, 0, 0")))

(fn CalculateReferenceCornerPosition
  (params (Wall :type FEWalls%20Enum) (Distance :type Integer) (XSize :type Float%20%28single-precision%29) (YSize :type Float%20%28single-precision%29) (Rotation :type FEFaces%20Enum) (OXSize :type Float%20%28single-precision%29) (OYSize :type Float%20%28single-precision%29) (Unit :type Float%20%28single-precision%29) (Width :type Float%20%28single-precision%29))
  (bind _returnvalue (/ OYSize 1.0))
  (bind _returnvalue_2 (/ OXSize 1.0))
  (bind _returnvalue_3 (* Distance Unit))
  (bind _objectfacetowall (CallFunction|CalculateFacetoWall Wall Rotation))
  (LocalVariables|SetLFaceToWall _objectfacetowall)
  (LocalVariables|SetLWidth Width)
  (switch Utilities|FlowControl|Switch|SwitchonFEFaces Rotation
    (:WallA
      ;[1 1 1] Objects dimensions after rotation
      (LocalVariables|SetLh _returnvalue_2 :!label _label)
      (LocalVariables|SetLv _returnvalue))
    (:WallB
      (LocalVariables|SetLh _returnvalue)
      (LocalVariables|SetLv _returnvalue_2))
    (:WallC
      (LocalVariables|SetLh _returnvalue_2)
      (LocalVariables|SetLv _returnvalue))
    (:WallD
      (LocalVariables|SetLh _returnvalue)
      (LocalVariables|SetLv _returnvalue_2))
    (:None
      (goto _label)))
  ;[1 1 1] Object position from wall face
  (switch Utilities|FlowControl|Switch|SwitchonFEWalls Wall
    (:WallA
      _)
    (:WallB
      (return (|(vector(((Xs-{D7AC1293-433E-638D-E6DB-6DA194327B6C})-{E67442D5-4461-1801-CA22-E38D52C5C7AE}),(Pos+{E67442D5-4461-1801-CA22-E38D52C5C7AE}),0)) XSize _returnvalue_3) (LocalVariables|GetLFaceToWall)))
    (:WallC
      (return (|(vector((((Xs-{E67442D5-4461-1801-CA22-E38D52C5C7AE})-Pos)-{D7AC1293-433E-638D-E6DB-6DA194327B6C}),((Ys-{E67442D5-4461-1801-CA22-E38D52C5C7AE})-{1668C1B7-40AA-83BF-11E9-73ACF0102542}),0)) XSize _returnvalue_3 YSize) (LocalVariables|GetLFaceToWall)))
    (:WallD
      (return (|(vector({E67442D5-4461-1801-CA22-E38D52C5C7AE},(((Ys-{E67442D5-4461-1801-CA22-E38D52C5C7AE})-Pos)-{1668C1B7-40AA-83BF-11E9-73ACF0102542}),0)) YSize _returnvalue_3) (LocalVariables|GetLFaceToWall)))
    (:None
      _))
  (return (|(vector((Pos+{E67442D5-4461-1801-CA22-E38D52C5C7AE}),{E67442D5-4461-1801-CA22-E38D52C5C7AE},0)) _returnvalue_3) (LocalVariables|GetLFaceToWall)))

(fn CalculateFacetoWall
  (params (Wall :type FEWalls%20Enum) (Rotation :type FEFaces%20Enum))
  (switch Utilities|FlowControl|Switch|SwitchonFEWalls Wall
    (:WallA
      (switch Utilities|FlowControl|Switch|SwitchonFEFaces Rotation :!label _label
        (:WallA
          _)
        (:WallB
          (return "WallB"))
        (:WallC
          (return "WallC"))
        (:WallD
          (return "WallD"))
        (:None
          _)))
    (:WallB
      (switch Utilities|FlowControl|Switch|SwitchonFEFaces Rotation
        (:WallA
          (return "WallB"))
        (:WallB
          (return "WallC"))
        (:WallC
          (return "WallD"))
        (:WallD
          _)
        (:None
          (return "WallB"))))
    (:WallC
      (switch Utilities|FlowControl|Switch|SwitchonFEFaces Rotation
        (:WallA
          (return "WallC"))
        (:WallB
          (return "WallD"))
        (:WallC
          _)
        (:WallD
          (return "WallB"))
        (:None
          (return "WallC"))))
    (:WallD
      (switch Utilities|FlowControl|Switch|SwitchonFEFaces Rotation
        (:WallA
          (return "WallD"))
        (:WallB
          _)
        (:WallC
          (return "WallB"))
        (:WallD
          (return "WallC"))
        (:None
          (return "WallD"))))
    (:None
      (goto _label)))
  (return "WallA"))

(fn GetStaticMeshComponentDimensions
  (params (SM%20Component :type Static%20Mesh%20Component%20Object%20Reference))
  (bind _returnvalue (Transformation|GetSocketLocation SM%20Component "PointF"))
  (bind _returnvalue_2 (Transformation|GetSocketLocation SM%20Component "Point1"))
  (bind _returnvalue_3 (Transformation|GetSocketLocation SM%20Component "Point2"))
  (bind _z (Math|Vector|BreakVector _returnvalue_2))
  (bind _returnvalue_4 (- _returnvalue_3 _returnvalue_2))
  (bind (_x _y) (Math|Vector|BreakVector _returnvalue))
  (bind (_x_2 _y_2 _z_2) (Math|Vector|BreakVector _returnvalue_4))
  (bind _returnvalue_5 (Math|Vector|MakeVector _x _y _z))
  (bind _returnvalue_6 (Math|Vector|MakeVector _x_2 _y_2 _z))
  (bind _returnvalue_7 (Math|Vector|GetUnitDirection(Vector) _returnvalue_2 _returnvalue_5))
  (return (Math|Vector|MakeVector (Math|Float|Absolute(Float) (Math|Vector|DotProduct _returnvalue_7 _returnvalue_6)) (Math|Float|Absolute(Float) (Math|Vector|DotProduct (Math|Vector|RotateVector _returnvalue_7 "0,90.000000, 0") _returnvalue_6)) (Math|Float|Absolute(Float) _z_2)) _returnvalue_7))